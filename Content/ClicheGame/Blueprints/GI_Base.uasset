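; Game instance that holds the current run's state: selected abilities, cliche abilities, map list and stage.
; On init it applies a fixed scalability level and ensures a global save exists.
; Run state is saved to and restored from a CurrentRun slot, refreshing pre-game widgets on load.
; Without a saved run it adds random maps, raising difficulty when an add leaves the list unchanged; ResetRun clears run state.
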(event `self.ReceiveInit`
  (bind _returnvalue (`GameUserSettings.GetGameUserSettings`))
  (`GameUserSettings.SetOverallScalabilityLevel` _returnvalue 2)
  (`GameUserSettings.ApplySettings` _returnvalue true)
  (bind _returnvalue_2 (`GameplayStatics.DoesSaveGameExist` "GlobalSave"))
  (if (not _returnvalue_2)
    (bind _returnvalue_3 (`GameplayStatics.CreateSaveGameObject` "/Game/ClicheGame/Blueprints/Data/Global_SaveGame.Global_SaveGame_C"))
    (`GameplayStatics.SaveGameToSlot` _returnvalue_3 "GlobalSave")))

(fn `InitSaveGame`
  (bind _returnvalue (`GameplayStatics.DoesSaveGameExist` "CurrentRun"))
  (if _returnvalue
    (bind _returnvalue_2 (`GameplayStatics.LoadGameFromSlot` "CurrentRun"))
    (bind _ascurrent_run_save_game (cast `/Game/ClicheGame/Blueprints/Data/CurrentRun_SaveGame` _returnvalue_2))
    (set `self.MapArray` (`/Game/ClicheGame/Blueprints/Data/CurrentRun_SaveGame.MapArray` _ascurrent_run_save_game))
    (set `self.SelectedAbilities` (`/Game/ClicheGame/Blueprints/Data/CurrentRun_SaveGame.SelectedAbilities` _ascurrent_run_save_game))
    (set `self.ClicheAbilities` (`/Game/ClicheGame/Blueprints/Data/CurrentRun_SaveGame.ClicheAbilities` _ascurrent_run_save_game))
    (set `self.CurrentStage` (`/Game/ClicheGame/Blueprints/Data/CurrentRun_SaveGame.CurrentStage` _ascurrent_run_save_game))
    (bind _foundwidgets (`WidgetBlueprintLibrary.GetAllWidgetsOfClass` "/Game/ClicheGame/Blueprints/UI/w_PreGame.w_PreGame_C" false))
    (for _array_element _foundwidgets
      (`/Game/ClicheGame/Blueprints/UI/w_PreGame.UpdateStats` _array_element (`self.SelectedAbilities`) (`self.ClicheAbilities`)))
    (else
      (`self.InitStages`))))

(fn `InitStages`
  (locals (CurrentDifficulty :type Integer) (MapSetSize :type Integer))
  (bind _maparray (`self.MapArray`))
  (set `local.CurrentDifficulty` 0)
  (set `local.MapSetSize` (`BlueprintSetLibrary.Set_Length` (`self.MapArray`)))
  (if (< (`local.MapSetSize`) 2)
    (for _ (range 2)
      (`BlueprintSetLibrary.Set_Add` _maparray (make `/Game/ClicheGame/Blueprints/Data/Stages_Struct` (select `int` (`KismetMathLibrary.RandomIntegerInRange` 0 4) :`0` "CaveMap" :`1` "CemeteryMap" :`2` "ForestMap" :`3` "SwampMap" :`4` "VillageMap") (`local.CurrentDifficulty`)) :!label _label)
      (if (== (`local.MapSetSize`) (`BlueprintSetLibrary.Set_Length` _maparray))
        (`/Engine/EditorBlueprintResources/StandardMacros.IncrementInt` (`local.CurrentDifficulty`)
          (:`  `
            (goto _label)))
        (else
          (set `local.CurrentDifficulty` 0)
          (set `local.MapSetSize` (`BlueprintSetLibrary.Set_Length` (`self.MapArray`))))))
    (else
      (goto _label))))

(fn `ResetRun`
  (bind _timeperstage (`self.TimePerStage`))
  (bind _selectedabilities (`self.SelectedAbilities`))
  (set `self.CurrentStage` 0)
  (set `self.Success?` false)
  (`|ExecutionSequence`
    (:`then_0`
      (for (_ _array_index) _timeperstage
        (`KismetArrayLibrary.Array_Set` _timeperstage _array_index)))
    (:`then_1`
      (for (_ _array_index_2) _selectedabilities
        (`KismetArrayLibrary.Array_Set` _selectedabilities _array_index_2 -1)))
    (:`then_2`
      (`KismetArrayLibrary.Array_Clear` (`self.ClicheAbilities`)))
    (:`then_3`
      (`BlueprintSetLibrary.Set_Clear` (`self.MapArray`)))))

(fn `SavePlayerRun`
  (bind _selectedabilities (`self.SelectedAbilities`))
  (bind _clicheabilities (`self.ClicheAbilities`))
  (bind _maparray (`self.MapArray`))
  (bind _currentstage (`self.CurrentStage`))
  (bind _returnvalue (`GameplayStatics.DoesSaveGameExist` "CurrentRun"))
  (if _returnvalue
    (bind _returnvalue_2 (`GameplayStatics.LoadGameFromSlot` "CurrentRun"))
    (bind _ascurrent_run_save_game (cast `/Game/ClicheGame/Blueprints/Data/CurrentRun_SaveGame` _returnvalue_2))
    (set `/Game/ClicheGame/Blueprints/Data/CurrentRun_SaveGame.SelectedAbilities` _selectedabilities _ascurrent_run_save_game)
    (set `/Game/ClicheGame/Blueprints/Data/CurrentRun_SaveGame.ClicheAbilities` _clicheabilities _ascurrent_run_save_game)
    (set `/Game/ClicheGame/Blueprints/Data/CurrentRun_SaveGame.MapArray` _maparray _ascurrent_run_save_game)
    (set `/Game/ClicheGame/Blueprints/Data/CurrentRun_SaveGame.CurrentStage` _currentstage _ascurrent_run_save_game)
    (`GameplayStatics.SaveGameToSlot` _returnvalue_2 "CurrentRun")
    (else
      (bind _returnvalue_3 (`GameplayStatics.CreateSaveGameObject` "/Game/ClicheGame/Blueprints/Data/CurrentRun_SaveGame.CurrentRun_SaveGame_C"))
      (set `/Game/ClicheGame/Blueprints/Data/CurrentRun_SaveGame.SelectedAbilities` _selectedabilities _returnvalue_3)
      (set `/Game/ClicheGame/Blueprints/Data/CurrentRun_SaveGame.ClicheAbilities` _clicheabilities _returnvalue_3)
      (set `/Game/ClicheGame/Blueprints/Data/CurrentRun_SaveGame.MapArray` _maparray _returnvalue_3)
      (set `/Game/ClicheGame/Blueprints/Data/CurrentRun_SaveGame.CurrentStage` _currentstage _returnvalue_3)
      (`GameplayStatics.SaveGameToSlot` _returnvalue_3 "CurrentRun"))))

(fn `UpdateSelectedAbility`
  (params (AbilitySlotIndex :type Integer) (AbilityIndex :type Integer))
  (`KismetArrayLibrary.Array_Set` (`self.SelectedAbilities`) AbilitySlotIndex AbilityIndex)
  (return))