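; Game mode for the swamp level, which spawns BP_SwampMonster near the player and finishes the level once enough enemies are killed.
; After the intro, a timer runs an EQS query and spawns a monster at a random result.
; SpawnSpeed is the delay in seconds: kills shorten it, while spawns and a passive timer lengthen it.
; Each spawn re-enters the setup, resetting both timers and adding another W_SwampUI.
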(event `self.EnemyKilled`
  (bind _enemieskilled (`self.EnemiesKilled`))
  (bind _spawnspeed (`self.SpawnSpeed`))
  (`/Engine/EditorBlueprintResources/StandardMacros.IncrementInt` _enemieskilled
    (:`  `
      (if (>= _enemieskilled (`self.KillsNeeded`))
        (`self.LevelFinished` true)
        (elif (<= _spawnspeed 3.0)
          (set `self.SpawnSpeed` 2.0)
          (else
            (set `self.SpawnSpeed` (- _spawnspeed 2.0))))))))

(event `self.ReceiveBeginPlay`
  (`parent.ReceiveBeginPlay`))

(event `self.IntroFinished`
  (`parent.IntroFinished`)
  (bind _returnvalue (`KismetSystemLibrary.K2_SetTimerDelegate` (delegate `SpawnEnemy`) (`self.SpawnSpeed`) true :!label _label))
  (`KismetSystemLibrary.K2_SetTimerDelegate` (delegate `PassiveDecreaseSpawnSpeed`) 30.0 true)
  (bind _returnvalue_2 (`|CreateWidget` "/Game/ClicheGame/Blueprints/UI/Levels/w_SwampUI.w_SwampUI_C" (`GameplayStatics.GetPlayerController` 0)))
  (`UserWidget.AddToViewport` _returnvalue_2 0))

(event `PassiveDecreaseSpawnSpeed`
  (`/Engine/EditorBlueprintResources/StandardMacros.IncrementFloat` (`self.SpawnSpeed`)))

(event `SpawnEnemy`
  (`KismetSystemLibrary.K2_ClearAndInvalidateTimerHandle` (stale `self.IntroFinished` _returnvalue))
  (bind _returnvalue (`EnvQueryManager.RunEQSQuery` "/Game/ClicheGame/Blueprints/Data/EQS_NearPlayerSpawn.EQS_NearPlayerSpawn" (`GameplayStatics.GetPlayerPawn` 0) "AllMatching"))
  (add `EnvQueryInstanceBlueprintWrapper.OnQueryFinishedEvent` _returnvalue (delegate `QueryFinished`))
  (`/Engine/EditorBlueprintResources/StandardMacros.IncrementFloat` (`self.SpawnSpeed`)))

(event `QueryFinished`
  (params (QueryInstance :type "EnvQueryInstanceBlueprintWrapper Object Reference") (QueryStatus :type "EEnvQueryStatus Enum" :default "Processing"))
  (bind _resultlocations (`EnvQueryInstanceBlueprintWrapper.GetQueryResultsAsLocations` (stale `SpawnEnemy` _returnvalue)))
  (`|SpawnActorFromClass` "/Game/ClicheGame/NPCs/Swamp_Monster/BP_SwampMonster.BP_SwampMonster_C" (`KismetMathLibrary.MakeTransform` (`KismetArrayLibrary.Array_Random` _resultlocations) (`KismetMathLibrary.MakeRotator` 0.0 0.0 (`KismetMathLibrary.RandomFloatInRange` 0.0 360.0))) "AdjustIfPossibleButAlwaysSpawn" "OverrideRootScale" null null)
  (goto _label))

(fn `UserConstructionScript`
  (`parent.UserConstructionScript`))