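; BP_Bomb is an ability bomb that explodes in a water splash when it hits anything other than the player pawn.
; On hit, it damages every actor overlapping ExplosionCollision, scaling Damage by the DamageBoost from the player character's C_AbilitySystem.
; It then spawns the explosion emitter, plays a splash sound with random volume and pitch, and destroys itself.
; An overlap-based trigger is present but disconnected.
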(event `self.ReceiveBeginPlay`
  (bind _asbp_cliche_character (cast `/Game/ClicheGame/Blueprints/BP_ClicheCharacter` (`GameplayStatics.GetPlayerPawn` 0)))
  (set `self.Character_Ref` _asbp_cliche_character))

(event `self.BombCollision.OnComponentHit`
  (params (HitComponent :type "PrimitiveComponent Object Reference") (OtherActor :type "Actor Object Reference") (OtherComp :type "PrimitiveComponent Object Reference") (NormalImpulse :type "Vector Structure") (Hit :type "HitResult Structure (by ref)"))
  (if (!= OtherActor (`GameplayStatics.GetPlayerPawn` 0))
    (for _array_element (`PrimitiveComponent.GetOverlappingActors` (`self.ExplosionCollision`) "/Script/Engine.Actor")
      (`GameplayStatics.ApplyDamage` _array_element (* (`KismetMathLibrary.Conv_IntToDouble` (`self.Damage`)) (`/Game/ClicheGame/Blueprints/Components/C_AbilitySystem.DamageBoost` (`self.GetComponentByClass` (`self.Character_Ref`) "/Game/ClicheGame/Blueprints/Components/C_AbilitySystem.C_AbilitySystem_C")))))
    (`GameplayStatics.SpawnEmitterAtLocation` "/Game/ClicheGame/Particles/Morigesh/Particles/Morigesh/Skins/NorthernMystic/P_Morigesh_NorthernMystic_SkillshotAOE_Explosion_Water.P_Morigesh_NorthernMystic_SkillshotAOE_Explosion_Water" (`self.K2_GetActorLocation`))
    (`GameplayStatics.PlaySoundAtLocation` "/Game/ClicheGame/Audio/SFX/Player/splash1.splash1" (`self.K2_GetActorLocation`) (struct) (`KismetMathLibrary.RandomFloatInRange` 0.7 0.9) (`KismetMathLibrary.RandomFloatInRange` 0.9 1.1) 0.0 "/Game/ClicheGame/Audio/SFX/Player/MediumDistanceAttenuation.MediumDistanceAttenuation" null null null)
    (`self.K2_DestroyActor`)))

(event `self.ReceiveTick`
  (params (DeltaSeconds :type "Float (single-precision)")))

(fn `UserConstructionScript`)