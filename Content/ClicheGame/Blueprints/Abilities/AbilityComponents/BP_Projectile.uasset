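; Player-fired ability projectile that damages whatever other actor it touches.
; BeginPlay caches the player's BP_ClicheCharacter.
; When its sphere overlaps anything except the player pawn, it applies its damage scaled by the DamageBoost on that character's C_AbilitySystem, credited to the player.
; It then spawns a hit particle and sound at its location and destroys itself.
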(event `self.ReceiveBeginPlay`
  (bind _asbp_cliche_character (cast `/Game/ClicheGame/Blueprints/BP_ClicheCharacter` (`GameplayStatics.GetPlayerPawn` 0)))
  (set `self.Character_Ref` _asbp_cliche_character))

(event `self.Sphere.OnComponentBeginOverlap`
  (params (OverlappedComponent :type "PrimitiveComponent Object Reference") (OtherActor :type "Actor Object Reference") (OtherComp :type "PrimitiveComponent Object Reference") (OtherBodyIndex :type Integer) (bFromSweep :type Boolean) (SweepResult :type "HitResult Structure (by ref)"))
  (if (!= (`GameplayStatics.GetPlayerPawn` 0) OtherActor)
    (`GameplayStatics.ApplyDamage` OtherActor (* (`KismetMathLibrary.Conv_IntToDouble` (`self.Damage`)) (`/Game/ClicheGame/Blueprints/Components/C_AbilitySystem.DamageBoost` (`self.GetComponentByClass` (`self.Character_Ref`) "/Game/ClicheGame/Blueprints/Components/C_AbilitySystem.C_AbilitySystem_C"))) (`GameplayStatics.GetPlayerController` 0) (`GameplayStatics.GetPlayerPawn` 0))
    (`GameplayStatics.SpawnEmitterAtLocation` "/Game/ClicheGame/Particles/Revenant/Particles/Revenant/Abilities/Primary/FX/P_Revenant_Primary_HitWorld.P_Revenant_Primary_HitWorld" (`self.K2_GetActorLocation`))
    (`GameplayStatics.PlaySoundAtLocation` "/Game/ClicheGame/Audio/SFX/Player/energy_hit.energy_hit" (`self.K2_GetActorLocation`) (struct) 0.8 1.0 0.0 "/Game/ClicheGame/Audio/SFX/Player/MediumDistanceAttenuation.MediumDistanceAttenuation" null null null)
    (`self.K2_DestroyActor`)))

(fn `UserConstructionScript`)