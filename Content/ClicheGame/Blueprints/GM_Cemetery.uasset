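; Game mode for the cemetery level, which finishes the level as a success once no skeletons are left.
; UpdateGraves waits a tick, then counts graves that still hold a skeleton plus live BP_Skeleton actors into SkeletonsLeft, calling LevelFinished at zero.
; The count runs on BeginPlay and whenever UpdateGraves is triggered.
; The cemetery UI widget is created after the parent's intro finishes.
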(event `self.ReceiveBeginPlay`
  (`parent.ReceiveBeginPlay`)
  (`self.UpdateGraves`))

(event `self.IntroFinished`
  (`parent.IntroFinished`)
  (bind _returnvalue (`|CreateWidget` "/Game/ClicheGame/Blueprints/UI/Levels/w_CemeteryUI.w_CemeteryUI_C" (`GameplayStatics.GetPlayerController` 0)))
  (`UserWidget.AddToViewport` _returnvalue 0)
  (set `self.CemeteryUI` _returnvalue))

(event `UpdateGraves`
  (`KismetSystemLibrary.DelayUntilNextTick`)
  (set `self.SkeletonsLeft` 0)
  (bind _outactors (`GameplayStatics.GetAllActorsOfClass` "/Game/ClicheGame/Environment/Cemetery/BP_Grave.BP_Grave_C"))
  (for _array_element _outactors
    (if (`/Game/ClicheGame/Environment/Cemetery/BP_Grave.DoesHaveSkeleton` _array_element)
      (`/Engine/EditorBlueprintResources/StandardMacros.IncrementInt` (`self.SkeletonsLeft`))))
  (bind _outactors_2 (`GameplayStatics.GetAllActorsOfClass` "/Game/ClicheGame/NPCs/Cemetery_Skeleton/BP_Skeleton.BP_Skeleton_C"))
  (set `self.SkeletonsLeft` (+ (`self.SkeletonsLeft`) (`KismetArrayLibrary.Array_Length` _outactors_2)))
  (if (== (`self.SkeletonsLeft`) 0)
    (`self.AllSkeletonsKilled`)))

(fn `AllSkeletonsKilled`
  (`self.LevelFinished` true))

(fn `UserConstructionScript`
  (`parent.UserConstructionScript`))