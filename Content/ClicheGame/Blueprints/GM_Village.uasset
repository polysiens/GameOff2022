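; Village level game mode that runs wave-based zombie combat and finishes the level once the last wave is cleared.
; After the intro it creates the village HUD, which shows wave changes and enemies left.
; Each kill recounts BP_NPC_Base actors a tick later; at zero, it advances the wave.
; An EQS query around the player supplies random spawn points for the zombie count in the Waves array.
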(event `self.ReceiveBeginPlay`
  (`parent.ReceiveBeginPlay`)
  (bind _outactors (`GameplayStatics.GetAllActorsOfClass` "/Game/ClicheGame/NPCs/BP_NPC_Base.BP_NPC_Base_C"))
  (set `self.EnemiesLeft` (`KismetArrayLibrary.Array_Length` _outactors)))

(event `self.IntroFinished`
  (`parent.IntroFinished`)
  (bind _returnvalue (`|CreateWidget` "/Game/ClicheGame/Blueprints/UI/Levels/w_VillageUI.w_VillageUI_C" (`GameplayStatics.GetPlayerController` 0)))
  (`UserWidget.AddToViewport` _returnvalue 0)
  (set `self.VillageUI_Ref` _returnvalue)
  (`/Game/ClicheGame/Blueprints/UI/Levels/w_VillageUI.NextWave` _returnvalue)
  (`/Game/ClicheGame/Blueprints/UI/Levels/w_VillageUI.UpdateEnemiesLeft` _returnvalue))

(event `self.EnemyKilled`
  (`KismetSystemLibrary.DelayUntilNextTick`)
  (`self.UpdateEnemiesLeftUI`)
  (if (== (`self.EnemiesLeft`) 0)
    (if (== (`self.CurrentWave`) (- (`KismetArrayLibrary.Array_Length` (`self.Waves`)) 1))
      (`self.LevelFinished` true)
      (else
        (`/Engine/EditorBlueprintResources/StandardMacros.IncrementInt` (`self.CurrentWave`)
          (:`  `
            (`/Game/ClicheGame/Blueprints/UI/Levels/w_VillageUI.NextWave` (`self.VillageUI_Ref`))
            (bind _returnvalue (`EnvQueryManager.RunEQSQuery` "/Game/ClicheGame/Blueprints/Data/EQSFindLocation.EQSFindLocation" (`GameplayStatics.GetPlayerPawn` 0) "AllMatching"))
            (add `EnvQueryInstanceBlueprintWrapper.OnQueryFinishedEvent` _returnvalue (delegate `SpawnLocations`))))))))

(event `SpawnLocations`
  (params (QueryInstance :type "EnvQueryInstanceBlueprintWrapper Object Reference") (QueryStatus :type "EEnvQueryStatus Enum" :default "Processing"))
  (bind _resultlocations (`EnvQueryInstanceBlueprintWrapper.GetQueryResultsAsLocations` (stale `self.EnemyKilled` _returnvalue)))
  (for _ (range 1 (+ (`|GetArrayItem` (`self.Waves`) (`self.CurrentWave`)) 1))
    (`|SpawnActorFromClass` "/Game/ClicheGame/NPCs/Village_Zombie/BP_Zombie.BP_Zombie_C" (`KismetMathLibrary.MakeTransform` (+ (`KismetArrayLibrary.Array_Random` _resultlocations) (0.0 0.0 100.0))) "Undefined" "OverrideRootScale" null null))
  (`self.UpdateEnemiesLeftUI`))

(fn `UpdateEnemiesLeftUI`
  (bind _outactors (`GameplayStatics.GetAllActorsOfClass` "/Game/ClicheGame/NPCs/BP_NPC_Base.BP_NPC_Base_C"))
  (set `self.EnemiesLeft` (`KismetArrayLibrary.Array_Length` _outactors))
  (`/Game/ClicheGame/Blueprints/UI/Levels/w_VillageUI.UpdateEnemiesLeft` (`self.VillageUI_Ref`)))

(fn `UserConstructionScript`
  (`parent.UserConstructionScript`))