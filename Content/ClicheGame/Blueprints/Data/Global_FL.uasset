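; Global function library with UI helpers for stage selection images and timer text.
; UpdateStageImages reads five GameInstance MapArray entries, switches on level name for icon and tooltip, defaulting to a locked padlock, and dims stages beyond CurrentStage.
; GetTime formats seconds as zero-padded MM:SS using TimeConverter's Minutes and Seconds, though TimeConverter's floor and modulo calculations appear here as unused nodes.
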(fn `GetTime`
  (params (TimerSeconds :type "Float (double-precision)"))
  (returns (ReturnValue :type String))
  (bind _returnvalue (`KismetMathLibrary.FFloor` (mod TimerSeconds 60.0)))
  (bind _returnvalue_2 (`KismetMathLibrary.FFloor` (/ TimerSeconds 60.0)))
  (bind _returnvalue_3 (`KismetStringLibrary.Conv_IntToString` _returnvalue_2))
  (bind _returnvalue_4 (`KismetStringLibrary.Conv_IntToString` _returnvalue))
  (return (`KismetStringLibrary.Concat_StrStr` (select `bool` (>= _returnvalue_2 10) :`false` (`KismetStringLibrary.Concat_StrStr` "0" _returnvalue_3) :`true` _returnvalue_3) ":" (select `bool` (>= _returnvalue 10) :`false` (`KismetStringLibrary.Concat_StrStr` "0" _returnvalue_4) :`true` _returnvalue_4))))

(fn `UpdateStageImages`
  (params (Image1 :type "Image Object Reference") (Image2 :type "Image Object Reference") (Image3 :type "Image Object Reference") (Image4 :type "Image Object Reference") (Image5 :type "Image Object Reference") (GameInstanceRef :type "/Game/ClicheGame/Blueprints/GI_Base Object Reference"))
  (locals (SetTexture :type "Texture Object Reference") (TooltipText :type Text))
  (for _index (range 5)
    (bind _result (`BlueprintSetLibrary.Set_ToArray` (`/Game/ClicheGame/Blueprints/GI_Base.MapArray` GameInstanceRef)))
    (bind _output_levelname (break `/Game/ClicheGame/Blueprints/Data/Stages_Struct` (`|GetArrayItem` _result _index)))
    (switch `string` _output_levelname
      (:`Default`
        (set `local.SetTexture` "/Game/ClicheGame/Blueprints/UI/Textures/Stages/PadlockIcon.PadlockIcon")
        (set `local.TooltipText` "Stage Locked."))
      (:`CaveMap`
        (set `local.SetTexture` "/Game/ClicheGame/Blueprints/UI/Textures/Stages/SpiderButton.SpiderButton")
        (set `local.TooltipText` "Kill Spiders to Gain points!"))
      (:`CemeteryMap`
        (set `local.SetTexture` "/Game/ClicheGame/Blueprints/UI/Textures/Stages/SkeletonButton.SkeletonButton")
        (set `local.TooltipText` "Destroy all the graves and skeletons that emerge!"))
      (:`ForestMap`
        (set `local.SetTexture` "/Game/ClicheGame/Blueprints/UI/Textures/Stages/WolfButton.WolfButton")
        (set `local.TooltipText` "Destroy 4 statues skattered across the map! Watch out for the wolves!"))
      (:`SwampMap`
        (set `local.SetTexture` "/Game/ClicheGame/Blueprints/UI/Textures/Stages/SwampButton.SwampButton")
        (set `local.TooltipText` "Destroy the incoming storm of swamp monsters!"))
      (:`VillageMap`
        (set `local.SetTexture` "/Game/ClicheGame/Blueprints/UI/Textures/Stages/ZombieButton.ZombieButton")
        (set `local.TooltipText` "Clear the waves of zombies in an overrun village!")))
    (bind _returnvalue (select `int` _index :`0` Image1 :`1` Image2 :`2` Image3 :`3` Image4 :`4` Image5))
    (`Image.SetBrush` _returnvalue (make `SlateBrush` (100.0 100.0) (struct) (make `SlateColor` (select `bool` (<= _index (`/Game/ClicheGame/Blueprints/GI_Base.CurrentStage` GameInstanceRef)) :`false` (struct :`R` 0.354167 :`G` 0.354167 :`B` 0.354167 :`A` 1.0) :`true` (struct :`R` 1.0 :`G` 1.0 :`B` 1.0 :`A` 1.0) :!type "LinearColor Structure")) (struct :`CornerRadii` (struct :`W` 1.0) :`Color` (struct :`SpecifiedColor` (struct) :`ColorUseRule` "UseColor_Specified") :`RoundingType` "HalfHeightRadius") (`local.SetTexture`)))
    (`Widget.SetToolTipText` _returnvalue (`local.TooltipText`))))