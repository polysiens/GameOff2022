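; Game mode for the forest level, which is won once no statues remain.
; After the intro it adds the forest UI and spawns wolves on a looping timer, capped by a wolf limit that a second timer keeps raising.
; Wolves spawn at random PlayerStarts, re-rolled to avoid the "Player"-tagged start and points near the player.
; UpdateStatues recounts statues a tick later to trigger the win.
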(event `self.ReceiveBeginPlay`
  (`parent.ReceiveBeginPlay`)
  (bind _outactors (`GameplayStatics.GetAllActorsOfClass` "/Game/ClicheGame/Environment/Forest/BP_Statue.BP_Statue_C"))
  (set `self.StatuesLeft` (`KismetArrayLibrary.Array_Length` _outactors)))

(event `self.IntroFinished`
  (`parent.IntroFinished`)
  (bind _returnvalue (`|CreateWidget` "/Game/ClicheGame/Blueprints/UI/Levels/w_ForestUI.w_ForestUI_C"))
  (`UserWidget.AddToViewport` _returnvalue 0)
  (`self.SpawnWolf`)
  (`KismetSystemLibrary.K2_SetTimerDelegate` (delegate `IncreseMaxWolves`) 40.0 true)
  (`KismetSystemLibrary.K2_SetTimerDelegate` (delegate `SpawnWolf`) 15.0 true))

(event `IncreseMaxWolves`
  (`/Engine/EditorBlueprintResources/StandardMacros.IncrementInt` (`self.MaxWolves`)))

(event `SpawnWolf`
  (bind _outactors (`GameplayStatics.GetAllActorsOfClass` "/Game/ClicheGame/NPCs/Forest_Wolf/BP_Wolf.BP_Wolf_C"))
  (if (< (`KismetArrayLibrary.Array_Length` _outactors) (`self.MaxWolves`))
    (bind _outactors_2 (`GameplayStatics.GetAllActorsOfClass` "/Script/Engine.PlayerStart" :!label _label))
    (bind _outitem (`KismetArrayLibrary.Array_Random` _outactors_2))
    (bind _output_get (set `self.StartActor` _outitem))
    (if (!= (`PlayerStart.PlayerStartTag` _outitem) "Player")
      (if (< (`KismetMathLibrary.Vector_Distance` (`self.K2_GetActorLocation` _output_get) (`self.K2_GetActorLocation` (`GameplayStatics.GetPlayerPawn` 0))) 8000.0)
        (goto _label)
        (else
          (`|SpawnActorFromClass` "/Game/ClicheGame/NPCs/Forest_Wolf/BP_Wolf.BP_Wolf_C" (`self.GetTransform` (`self.StartActor`)) "AdjustIfPossibleButAlwaysSpawn" "OverrideRootScale" null null)))
      (else
        (goto _label)))))

(event `UpdateStatues`
  (`KismetSystemLibrary.DelayUntilNextTick`)
  (bind _outactors (`GameplayStatics.GetAllActorsOfClass` "/Game/ClicheGame/Environment/Forest/BP_Statue.BP_Statue_C"))
  (set `self.StatuesLeft` (`KismetArrayLibrary.Array_Length` _outactors))
  (if (== (`self.StatuesLeft`) 0)
    (`self.LevelFinished` true)))

(fn `FindPlayerStart`
  (params (Player :type "Controller Object Reference") (IncomingName :type String))
  (returns (ReturnValue :type "Actor Object Reference"))
  (bind _outactors (`GameplayStatics.GetAllActorsOfClass` "/Script/Engine.PlayerStart"))
  (for _array_element _outactors
    (if (== (`PlayerStart.PlayerStartTag` _array_element) "Player")
      (return _array_element))))

(fn `UserConstructionScript`
  (`parent.UserConstructionScript`))