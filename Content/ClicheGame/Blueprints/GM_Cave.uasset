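; Game mode for the cave level, which spawns spiders at random intervals and finishes the level successfully when the score reaches 100.
; After the intro, it adds W_CaveUI and starts a 2–8 second random timer.
; Each BP_Spider teleports to Player Starts matching its colour ("Red" tag or otherwise), looping back to re-roll the timer and create another UI widget.
; FindPlayerStart is overridden to return a start tagged "None".
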(event `self.IntroFinished`
  (`parent.IntroFinished`)
  (bind _returnvalue (`KismetSystemLibrary.K2_SetTimerDelegate` (delegate `SpawnSpiders`) (`KismetMathLibrary.RandomFloatInRange` 2.0 8.0) true :!label _label))
  (bind _returnvalue_2 (`|CreateWidget` "/Game/ClicheGame/Blueprints/UI/Levels/w_CaveUI.w_CaveUI_C" (`GameplayStatics.GetPlayerController` 0)))
  (`UserWidget.AddToViewport` _returnvalue_2 0))

(event `SpawnSpiders`
  (`KismetSystemLibrary.K2_ClearAndInvalidateTimerHandle` (stale `self.IntroFinished` _returnvalue))
  (bind _returnvalue (`|SpawnActorFromClass` "/Game/ClicheGame/NPCs/Cave_Spider/BP_Spider.BP_Spider_C" (`KismetMathLibrary.MakeTransform` (0.0 0.0 0.0)) "AlwaysSpawn" "OverrideRootScale" null null))
  (bind _outactors (`GameplayStatics.GetAllActorsOfClass` "/Script/Engine.PlayerStart"))
  (for _array_element _outactors
    (if (== (`PlayerStart.PlayerStartTag` _array_element) "Red")
      (bind _isredspider_ (`/Game/ClicheGame/NPCs/Cave_Spider/BP_Spider.IsRedSpider?` _returnvalue))
      (if _isredspider_
        (`self.K2_SetActorLocationAndRotation` _returnvalue (`self.K2_GetActorLocation` _array_element) (`self.K2_GetActorRotation` _array_element) false true :!label _label_2)
        (goto _label))
      (elif (not _isredspider_)
        (goto _label_2)))))

(event `IncreaseScore`
  (params (IncreaseScore :type Integer))
  (set `self.Score` (+ (`self.Score`) IncreaseScore))
  (if (>= (`self.Score`) 100)
    (`self.LevelFinished` true)))

(fn `FindPlayerStart`
  (params (Player :type "Controller Object Reference") (IncomingName :type String))
  (returns (ReturnValue :type "Actor Object Reference"))
  (bind _outactors (`GameplayStatics.GetAllActorsOfClass` "/Script/Engine.PlayerStart"))
  (for _array_element _outactors
    (if (== (`PlayerStart.PlayerStartTag` _array_element) "None")
      (return _array_element))))

(fn `UserConstructionScript`
  (`parent.UserConstructionScript`))