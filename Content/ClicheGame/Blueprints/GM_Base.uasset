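; Base game mode that runs one timed stage of a multi-stage run, from intro to result.
; BeginPlay plays an intro sequence, then creates the timer and player UI and starts a one-second tick that fails the stage after ten minutes.
; LevelFinished runs once, shows a pop-up, and on success records the time in GI_Base and the CurrentRun save.
; It then opens GameMenu, or EndGameMenu on failure or final-stage completion.
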(event `self.ReceiveBeginPlay`
  (`WidgetBlueprintLibrary.SetInputMode_GameOnly` (`GameplayStatics.GetPlayerController` 0))
  (bind (_outactor _returnvalue) (`LevelSequencePlayer.CreateLevelSequencePlayer` (`self.IntroSequence`) (make `MovieSceneSequencePlaybackSettings` true (make `MovieSceneSequenceLoopCount` 0) 1.0 0.0 false false true true false true)))
  (`/Engine/EditorBlueprintResources/StandardMacros.IsValid` _returnvalue
    (:`Is Valid`
      (add `MovieSceneSequencePlayer.OnFinished` _returnvalue (delegate `IntroFinished`)))
    (:`Is Not Valid`
      (bind _returnvalue_2 (`|CreateWidget` "/Game/ClicheGame/Blueprints/UI/w_GameTimer.w_GameTimer_C" (`GameplayStatics.GetPlayerController` 0) :!label _label))
      (`UserWidget.AddToViewport` _returnvalue_2 0)
      (bind _returnvalue_3 (`KismetSystemLibrary.K2_SetTimerDelegate` (delegate `TimerTick`) 1.0 true))
      (bind _aspc_base (cast `/Game/ClicheGame/Blueprints/PC_base` (`GameplayStatics.GetPlayerController` 0)))
      (`/Game/ClicheGame/Blueprints/PC_base.CreatePlayerUI` _aspc_base))))

(event `IntroFinished`
  (goto _label))

(event `TimerTick`
  (bind _timerseconds (`self.TimerSeconds`))
  (`/Engine/EditorBlueprintResources/StandardMacros.IncrementFloat` _timerseconds
    (:`  `
      (if (> _timerseconds 600.0)
        (`self.LevelFinished` false)))))

(event `LevelFinished`
  (params (`Success?` :type Boolean))
  (bind _gi_base_ref (`self.GI_Base_Ref`))
  (bind _gi_base_ref_2 (`self.GI_Base_Ref`))
  (bind _gi_base_ref_3 (`self.GI_Base_Ref`))
  (bind _currentstage (`/Game/ClicheGame/Blueprints/GI_Base.CurrentStage` _gi_base_ref_3))
  (`/Engine/EditorBlueprintResources/StandardMacros.DoOnce` false
    (:`Completed`
      (`KismetSystemLibrary.K2_ClearAndInvalidateTimerHandle` (stale `self.ReceiveBeginPlay` _returnvalue_3))
      (bind _returnvalue (`|CreateWidget` "/Game/ClicheGame/Blueprints/UI/w_endGamePopUp.w_endGamePopUp_C" (`GameplayStatics.GetPlayerController` 0) `Success?`))
      (`UserWidget.AddToViewport` _returnvalue 0)
      (`KismetSystemLibrary.Delay` 3.0)
      (bind _asgi_base (cast `/Game/ClicheGame/Blueprints/GI_Base` (`GameplayStatics.GetGameInstance`)))
      (set `self.GI_Base_Ref` _asgi_base)
      (if `Success?`
        (`KismetArrayLibrary.Array_Set` (`/Game/ClicheGame/Blueprints/GI_Base.TimePerStage` _gi_base_ref_3) _currentstage (`self.TimerSeconds`))
        (set `/Game/ClicheGame/Blueprints/GI_Base.CurrentStage` (+ _currentstage 1) _gi_base_ref)
        (bind _returnvalue_2 (`GameplayStatics.LoadGameFromSlot` "CurrentRun"))
        (bind _ascurrent_run_save_game (cast `/Game/ClicheGame/Blueprints/Data/CurrentRun_SaveGame` _returnvalue_2)
          (:`then`
            (`KismetArrayLibrary.Array_Set` (`/Game/ClicheGame/Blueprints/Data/CurrentRun_SaveGame.TImePerStage` _ascurrent_run_save_game) (`/Game/ClicheGame/Blueprints/GI_Base.CurrentStage` _gi_base_ref) (`self.TimerSeconds`))
            (`GameplayStatics.SaveGameToSlot` _returnvalue_2 "CurrentRun"))
          (:`CastFailed`
            _))
        (if (> (`/Game/ClicheGame/Blueprints/GI_Base.CurrentStage` _gi_base_ref_2) 4)
          (set `/Game/ClicheGame/Blueprints/GI_Base.Success?` true (`self.GI_Base_Ref`))
          (`GameplayStatics.OpenLevel` "EndGameMenu")
          (else
            (`/Game/ClicheGame/Blueprints/GI_Base.InitStages` _gi_base_ref_2)
            (`/Game/ClicheGame/Blueprints/GI_Base.SavePlayerRun` _gi_base_ref_2)
            (`GameplayStatics.OpenLevel` "GameMenu")))
        (else
          (set `/Game/ClicheGame/Blueprints/GI_Base.Success?` false (`self.GI_Base_Ref`))
          (`GameplayStatics.OpenLevel` "EndGameMenu"))))))

(fn `EnemyKilled`)

(fn `UserConstructionScript`)