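; C_Developer is a debug component that binds number-key cheats for testing the game.
; On BeginPlay it caches the player BP_ClicheCharacter and its walk speed.
; Keys 1–3 destroy all NPCs and graves, set player health to full and toggle a speed boost through a FlipFlop.
; Keys 4–5 call LevelFinished on GM_Base with true or false, and key 6 resets the ability system's use amounts.
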(event `self.ReceiveBeginPlay`
  (bind _asbp_cliche_character (cast `/Game/ClicheGame/Blueprints/BP_ClicheCharacter` (`GameplayStatics.GetPlayerPawn` 0)))
  (set `self.Char_Ref` _asbp_cliche_character)
  (set `self.MovementSpeed` (`CharacterMovementComponent.MaxWalkSpeed` (`Character.CharacterMovement` (`self.Char_Ref`)))))

(event `Key|One`
  (params (Key :type "Key Structure"))
  (:`Pressed`
    (bind _outactors (`GameplayStatics.GetAllActorsOfClass` "/Game/ClicheGame/NPCs/BP_NPC_Base.BP_NPC_Base_C"))
    (for _array_element _outactors
      (`Actor.K2_DestroyActor` _array_element))
    (bind _outactors_2 (`GameplayStatics.GetAllActorsOfClass` "/Game/ClicheGame/Environment/Cemetery/BP_Grave.BP_Grave_C"))
    (for _array_element_2 _outactors_2
      (`Actor.K2_DestroyActor` _array_element_2))))

(event `Key|Two`
  (params (Key :type "Key Structure"))
  (:`Pressed`
    (set `/Game/ClicheGame/Blueprints/BP_ClicheCharacter.Health` 100 (`self.Char_Ref`))))

(event `Key|Three`
  (params (Key :type "Key Structure"))
  (bind _charactermovement (`Character.CharacterMovement` (`self.Char_Ref`)))
  (:`Pressed`
    (`/Engine/EditorBlueprintResources/StandardMacros.FlipFlop`
      (:`A`
        (set `CharacterMovementComponent.MaxWalkSpeed` 1500.0 _charactermovement))
      (:`B`
        (set `CharacterMovementComponent.MaxWalkSpeed` (`self.MovementSpeed`) _charactermovement)))))

(event `Key|Four`
  (params (Key :type "Key Structure"))
  (:`Pressed`
    (bind _asgm_base (cast `/Game/ClicheGame/Blueprints/GM_Base` (`GameplayStatics.GetGameMode`)))
    (`/Game/ClicheGame/Blueprints/GM_Base.LevelFinished` _asgm_base true)))

(event `Key|Five`
  (params (Key :type "Key Structure"))
  (:`Pressed`
    (bind _asgm_base (cast `/Game/ClicheGame/Blueprints/GM_Base` (`GameplayStatics.GetGameMode`)))
    (`/Game/ClicheGame/Blueprints/GM_Base.LevelFinished` _asgm_base false)))

(event `Key|Six`
  (params (Key :type "Key Structure"))
  (:`Pressed`
    (bind _asbp_cliche_character (cast `/Game/ClicheGame/Blueprints/BP_ClicheCharacter` (`GameplayStatics.GetPlayerPawn` 0)))
    (bind _abilityuseamount (`/Game/ClicheGame/Blueprints/Components/C_AbilitySystem.AbilityUseAmount` (`/Game/ClicheGame/Blueprints/BP_ClicheCharacter.C_AbilitySystem` _asbp_cliche_character)))
    (for (_ _array_index) _abilityuseamount
      (`KismetArrayLibrary.Array_Set` _abilityuseamount _array_index))))