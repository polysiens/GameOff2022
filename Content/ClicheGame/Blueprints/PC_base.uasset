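; Base player controller for ClicheGame that handles the pause menu and player HUD creation.
; Escape shows W_PauseMenu, using an existing top-level instance if found or creating one, then sets UI-only input and shows the cursor, without pausing the game itself.
; CreatePlayerUI adds W_PlayerUI to the viewport and stores its reference, but nothing in this Blueprint calls it.
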(event `Key|Escape`
  (params (Key :type "Key Structure"))
  (bind _returnvalue (`GameplayStatics.GetPlayerController` 0))
  (:`Pressed`
    (bind _foundwidgets (`WidgetBlueprintLibrary.GetAllWidgetsOfClass` "/Game/ClicheGame/Blueprints/UI/w_PauseMenu.w_PauseMenu_C"))
    (if (> (`KismetArrayLibrary.Array_Length` _foundwidgets) 0)
      (bind _output (`|GetArrayItem` _foundwidgets))
      (`UserWidget.AddToViewport` _output 0)
      (`WidgetBlueprintLibrary.SetInputMode_UIOnlyEx` _returnvalue _output)
      (else
        (bind _returnvalue_2 (`|CreateWidget` "/Game/ClicheGame/Blueprints/UI/w_PauseMenu.w_PauseMenu_C"))
        (`UserWidget.AddToViewport` _returnvalue_2 0)
        (`WidgetBlueprintLibrary.SetInputMode_UIOnlyEx` (`GameplayStatics.GetPlayerController` 0) _returnvalue_2)))
    (set `PlayerController.bShowMouseCursor` true _returnvalue)))

(fn `CreatePlayerUI`
  (bind _returnvalue (`|CreateWidget` "/Game/ClicheGame/Blueprints/UI/w_PlayerUI.w_PlayerUI_C"))
  (`UserWidget.AddToViewport` _returnvalue 0)
  (set `self.PlayerUI_Ref` _returnvalue))

(fn `UserConstructionScript`)