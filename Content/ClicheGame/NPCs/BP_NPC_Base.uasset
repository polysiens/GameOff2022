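; Base NPC character with health, player perception and a floating widget.
; Perception updates about the player write the stimulus location to the blackboard as PlayerLocation.
; Damage reduces health and, at zero, calls the empty DiesEffect event and flags the dying state, while IncreaseHealth heals up to MaxHealth.
; The widget turns toward the player every tick, a looping timer shows it only within range, and landing sets the capsule to block Pawns.
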(event `self.ReceiveBeginPlay`
  (`|ExecutionSequence`
    (:`then_0`
      (add `AIPerceptionComponent.OnTargetPerceptionUpdated` (`self.AIPerception`) (delegate `OnTargetPerceptionUpdated`))
      (bind _asaic_base (cast `/Game/ClicheGame/NPCs/AIC_Base` (`self.GetController`)))
      (set `self.AIController_Ref` _asaic_base)
      (set `self.PlayerPawn_Ref` (`GameplayStatics.GetPlayerPawn` 0)))
    (:`then_1`
      (bind _asw_npc_widget (cast `/Game/ClicheGame/Blueprints/UI/w_NPC_Widget` (`WidgetComponent.GetWidget` (`self.NPC_Widget`))))
      (set `/Game/ClicheGame/Blueprints/UI/w_NPC_Widget.NPC_Ref` self _asw_npc_widget))
    (:`then_2`
      (`KismetSystemLibrary.K2_SetTimerDelegate` (delegate `UpdateWidgetVisibility`) 0.5 true))))

(event `self.ReceiveAnyDamage`
  (params (Damage :type "Float (single-precision)") (DamageType :type "DamageType Object Reference") (InstigatedBy :type "Controller Object Reference") (DamageCauser :type "Actor Object Reference"))
  (bind _health (`self.Health`))
  (set `self.Health` (`KismetMathLibrary.FTrunc` (- _health Damage)))
  (if (<= _health 0)
    (`KismetSystemLibrary.DelayUntilNextTick`)
    (`self.DiesEffect`)
    (set `self.InDyingState?` true)))

(event `OnTargetPerceptionUpdated`
  (params (Actor :type "Actor Object Reference") (Stimulus :type "AIStimulus Structure"))
  (if (== Actor (`self.PlayerPawn_Ref`))
    (`BlackboardComponent.SetValueAsVector` (`AIBlueprintHelperLibrary.GetBlackboard` null) "PlayerLocation" Stimulus_StimulusLocation)))

(event `DiesEffect`)

(event `self.OnLanded`
  (params (Hit :type "HitResult Structure (by ref)"))
  (`PrimitiveComponent.SetCollisionResponseToChannel` (`self.CapsuleComponent`) "ECC_Pawn" "ECR_Block"))

(event `self.ReceiveTick`
  (params (DeltaSeconds :type "Float (single-precision)"))
  (bind _returnvalue (`GameplayStatics.GetPlayerPawn` 0))
  (`/Engine/EditorBlueprintResources/StandardMacros.IsValid` _returnvalue
    (:`Is Valid`
      (`SceneComponent.K2_SetWorldRotation` (`self.NPC_Widget`) (`KismetMathLibrary.FindLookAtRotation` (`self.K2_GetActorLocation`) (`self.K2_GetActorLocation` _returnvalue)) false false))))

(event `UpdateWidgetVisibility`
  (`SceneComponent.SetVisibility` (`self.NPC_Widget`) (< (`KismetMathLibrary.Vector_Distance` (`self.K2_GetActorLocation`) (`self.K2_GetActorLocation` (`GameplayStatics.GetPlayerPawn` 0))) 6000.0) false))

(fn `IncreaseHealth`
  (params (HealthAmount :type Integer))
  (bind _returnvalue (+ HealthAmount (`self.Health`)))
  (if (> _returnvalue (`self.MaxHealth`))
    (set `self.Health` (`self.MaxHealth`))
    (else
      (set `self.Health` _returnvalue))))

(fn `UserConstructionScript`)