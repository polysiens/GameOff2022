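; BP_Zombie is a village zombie NPC that layers sound, nameplate color and death behavior onto its parent class.
; A finished-audio callback and retriggerable random delay loop roaming groans through one audio component, while damage randomly triggers hit sounds.
; A one-shot death effect stops AI logic, plays the death animation and sound, then spawns a particle burst and flesh pile before destroying the actor.
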(event `self.ReceiveAnyDamage`
  (params (Damage :type "Float (single-precision)") (DamageType :type "DamageType Object Reference") (InstigatedBy :type "Controller Object Reference") (DamageCauser :type "Actor Object Reference"))
  (bind _zombiesounds (`self.ZombieSounds`))
  (`parent.ReceiveAnyDamage` Damage DamageType InstigatedBy DamageCauser)
  (if (and (> (`KismetMathLibrary.RandomFloatInRange` 0.0 1.0) 0.4) (not (`self.InDyingState?`)))
    (`KismetSystemLibrary.Delay` (`KismetMathLibrary.RandomFloatInRange` 0.0 0.2))
    (`AudioComponent.SetSound` (`self.ZombieSounds`) "/Game/ClicheGame/Audio/SFX/Zombie/ZombieHit/Cue_ZombieHit.Cue_ZombieHit")
    (`GameplayStatics.PlaySoundAtLocation` (`AudioComponent.Sound` _zombiesounds) (`self.K2_GetActorLocation`) (struct) 0.2 1.0 0.0 "/Game/ClicheGame/Audio/SFX/DefaultAttenuation.DefaultAttenuation" null null null)
    (`AudioComponent.FadeIn` _zombiesounds 0.5 (`KismetMathLibrary.RandomFloatInRange` 0.1 0.3) 0.0 "Linear")))

(event `self.ReceiveBeginPlay`
  (`parent.ReceiveBeginPlay`)
  (bind _asw_npc_widget (cast `/Game/ClicheGame/Blueprints/UI/w_NPC_Widget` (`WidgetComponent.GetWidget` (`self.NPC_Widget`))))
  (`/Game/ClicheGame/Blueprints/UI/w_NPC_Widget.SetColor` _asw_npc_widget (struct :`R` 0.035601 :`G` 0.254152 :`B` 0.015996 :`A` 1.0))
  (add `AudioComponent.OnAudioFinished` (`self.ZombieSounds`) (delegate `OnAudioFinished`))
  (`self.RetriggerSound`))

(event `OnAudioFinished`
  (bind _zombiesounds (`self.ZombieSounds`))
  (`KismetSystemLibrary.RetriggerableDelay` (`KismetMathLibrary.RandomFloatInRange` 0.0 5.0) :!label _label)
  (`AudioComponent.SetSound` (`self.ZombieSounds`) "/Game/ClicheGame/Audio/SFX/Zombie/ZombieRoaming/Cue_ZombieRoaming.Cue_ZombieRoaming")
  (`AudioComponent.Play` _zombiesounds 0.0)
  (`AudioComponent.SetVolumeMultiplier` _zombiesounds 0.3))

(event `RetriggerSound`
  (goto _label))

(event `self.DiesEffect`
  (bind (_returnvalue_x _returnvalue_y _returnvalue_z) (`KismetMathLibrary.BreakVector` (`self.K2_GetActorLocation`)))
  (bind _mesh (`self.Mesh`))
  (`/Engine/EditorBlueprintResources/StandardMacros.DoOnce` false
    (:`Completed`
      (`BrainComponent.StopLogic` (`AIController.BrainComponent` (`self.AIController_Ref`)) "")
      (`SkeletalMeshComponent.SetAnimationMode` _mesh "AnimationSingleNode")
      (`SkeletalMeshComponent.PlayAnimation` _mesh "/Game/ClicheGame/NPCs/Village_Zombie/Animations/Anim_Death.Anim_Death" false)
      (`SceneComponent.K2_AddWorldOffset` (`self.Mesh`) (* (* (`self.GetActorForwardVector`) -1) 50) false false)
      (`self.DiesSound`)
      (`KismetSystemLibrary.Delay` 1.5)
      (`GameplayStatics.SpawnEmitterAtLocation` "/Game/ClicheGame/Particles/Morigesh/Particles/Morigesh/Abilities/SkillshotAOE/FX/P_Morigesh_DOT_Impact.P_Morigesh_DOT_Impact" (`KismetMathLibrary.MakeVector` _returnvalue_x _returnvalue_y (- _returnvalue_z 60.0)) (struct) (3.0 3.0 3.0))
      (`KismetSystemLibrary.Delay` 0.15)
      (`|SpawnActorFromClass` "/Game/ClicheGame/NPCs/Village_Zombie/BP_FleshPile.BP_FleshPile_C" (`self.GetTransform`) "AlwaysSpawn" "OverrideRootScale" null null)
      (`self.K2_DestroyActor`))))

(fn `DiesSound`
  (bind _zombiesounds (`self.ZombieSounds`))
  (`AudioComponent.SetSound` _zombiesounds "/Game/ClicheGame/Audio/SFX/Zombie/Cue_Zombie_Death.Cue_Zombie_Death")
  (`AudioComponent.SetVolumeMultiplier` _zombiesounds 0.3)
  (`AudioComponent.Play` _zombiesounds 0.0))

(fn `UserConstructionScript`
  (`parent.UserConstructionScript`))