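; BP_FleshPile is a destructible flesh pile actor from the Village Zombie NPC set.
; On BeginPlay it traces straight down against WorldStatic objects and moves itself to the first impact point, snapping to the ground.
; DecreaseHealth subtracts a given amount from Health and destroys the actor once it reaches zero or below.
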(event `self.ReceiveBeginPlay`
  (bind _returnvalue (`self.K2_GetActorLocation`))
  (bind (_outhits _returnvalue_2) (`KismetSystemLibrary.LineTraceMultiForObjects` _returnvalue (+ _returnvalue (0.0 0.0 -10000.0)) (`|MakeArray` "ObjectTypeQuery1" :!type "EObjectTypeQuery Enum")))
  (if _returnvalue_2
    (bind (_output_bblockinghit _output_binitialoverlap _output_time _output_distance _output_location _output_impactpoint) (`GameplayStatics.BreakHitResult` (`|GetArrayItem` _outhits)))
    (`self.K2_SetActorLocation` _output_impactpoint)))

(fn `DecreaseHealth`
  (params (HealthAmount :type Integer))
  (bind _output_get (set `self.Health` (- (`self.Health`) HealthAmount)))
  (if (<= _output_get 0)
    (`self.K2_DestroyActor`)))

(fn `UserConstructionScript`)