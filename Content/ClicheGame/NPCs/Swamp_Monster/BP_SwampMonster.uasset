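; Swamp monster NPC Blueprint that handles its spawn and death presentation on top of inherited NPC behavior.
; On BeginPlay it halts AI movement, plays a tripped alert animation from an offset, then switches to its Animation Blueprint, while also tinting its NPC widget.
; DiesEffect reports the kill to GM_Swamp, plays the death animation, spawns a particle effect and destroys the actor after short delays.
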(event `self.ReceiveBeginPlay`
  (bind _mesh (`self.Mesh`))
  (bind _mesh_2 (`self.Mesh`))
  (`parent.ReceiveBeginPlay`)
  (`|ExecutionSequence`
    (:`then_0`
      (`Controller.StopMovement` (`self.AIController_Ref`))
      (`SkeletalMeshComponent.SetAnimationMode` _mesh_2 "AnimationSingleNode")
      (`SkeletalMeshComponent.SetAnimation` _mesh_2 "/Game/ClicheGame/NPCs/Cemetery_Skeleton/Animation/Corpse_Alert_Tripped.Corpse_Alert_Tripped")
      (`SkeletalMeshComponent.SetPosition` _mesh_2 2.0 true)
      (`SkeletalMeshComponent.Play` _mesh_2 false)
      (`KismetSystemLibrary.Delay` 1.3)
      (`SkeletalMeshComponent.SetAnimationMode` _mesh "AnimationBlueprint")
      (`SkeletalMeshComponent.SetAnimInstanceClass` _mesh "/Game/ClicheGame/NPCs/Swamp_Monster/ABP_SwampMonster.ABP_SwampMonster_C"))
    (:`then_1`
      (bind _asw_npc_widget (cast `/Game/ClicheGame/Blueprints/UI/w_NPC_Widget` (`WidgetComponent.GetWidget` (`self.NPC_Widget`))))
      (`/Game/ClicheGame/Blueprints/UI/w_NPC_Widget.SetColor` _asw_npc_widget (struct :`R` 0.135633 :`G` 0.23074 :`B` 0.584079 :`A` 1.0)))))

(event `self.DiesEffect`
  (bind _mesh (`self.Mesh`))
  (bind _asgm_swamp (cast `/Game/ClicheGame/Blueprints/GM_Swamp` (`GameplayStatics.GetGameMode`))
    (:`then`
      (`/Game/ClicheGame/Blueprints/GM_Base.EnemyKilled` _asgm_swamp))
    (:`CastFailed`
      _))
  (`SkeletalMeshComponent.SetAnimationMode` _mesh "AnimationSingleNode")
  (`SkeletalMeshComponent.PlayAnimation` _mesh "/Game/ClicheGame/NPCs/Cemetery_Skeleton/Animation/Corpse_Alert_Death.Corpse_Alert_Death" false)
  (`KismetSystemLibrary.Delay` 0.5)
  (`GameplayStatics.SpawnEmitterAtLocation` "/Game/ClicheGame/NPCs/Swamp_Monster/p_swamp_monsterDeath.p_swamp_monsterDeath" (`self.K2_GetActorLocation`))
  (`KismetSystemLibrary.Delay` 0.1)
  (`self.K2_DestroyActor`))

(fn `UserConstructionScript`
  (`parent.UserConstructionScript`))