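; Cave spider NPC that spawns as a randomly chosen red or non-red mesh variant with random health, and awards points to the cave game mode when it dies.
; At 25% health or less it sets a blackboard flag to activate its special.
; On death it plays an effect and scores by the first overlapping trigger volume: more for a matching Red or Green tag, less otherwise, none without a volume.
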(event `self.ReceiveBeginPlay`
  (bind _mesh (`self.Mesh`))
  (`parent.ReceiveBeginPlay`)
  (`|ExecutionSequence`
    (:`then_0`
      (set `self.GM_Cave_Ref` (cast `/Game/ClicheGame/Blueprints/GM_Cave` (`GameplayStatics.GetGameMode`) :!pure true))
      (bind _output_get (set `self.Health` (`KismetMathLibrary.RandomIntegerInRange` 80 100)))
      (set `self.MaxHealth` _output_get)
      (bind _output_get_2 (set `self.IsRedSpider?` (`KismetMathLibrary.RandomBool`)))
      (if _output_get_2
        (`SkinnedMeshComponent.SetSkinnedAssetAndUpdate` _mesh "/Game/ClicheGame/NPCs/Cave_Spider/Enemy_Greater_Spider_Boss/SK_Greater_Spider_Boss_Cine.SK_Greater_Spider_Boss_Cine" false)
        (else
          (`SkinnedMeshComponent.SetSkinnedAssetAndUpdate` _mesh "/Game/ClicheGame/NPCs/Cave_Spider/Enemy_Greater_Spider_Boss/SK_Greater_Spider_Boss.SK_Greater_Spider_Boss" false))))
    (:`then_1`
      (bind _asw_npc_widget (cast `/Game/ClicheGame/Blueprints/UI/w_NPC_Widget` (`WidgetComponent.GetWidget` (`self.NPC_Widget`))))
      (`/Game/ClicheGame/Blueprints/UI/w_NPC_Widget.SetColor` _asw_npc_widget (struct :`R` 0.361307 :`G` 0.07036 :`B` 0.07036 :`A` 1.0)))))

(event `self.DiesEffect`
  (`GameplayStatics.SpawnEmitterAtLocation` "/Game/ClicheGame/Particles/FengMao/Particles/Abilities/Block/FX/PS_FengMao_AttackBuff.PS_FengMao_AttackBuff" (`self.K2_GetActorLocation`) (struct) (3.0 3.0 3.0))
  (`self.EvaluateScore`)
  (`self.K2_DestroyActor`))

(event `self.ReceiveAnyDamage`
  (params (Damage :type "Float (single-precision)") (DamageType :type "DamageType Object Reference") (InstigatedBy :type "Controller Object Reference") (DamageCauser :type "Actor Object Reference"))
  (`parent.ReceiveAnyDamage` Damage DamageType InstigatedBy DamageCauser)
  (if (<= (/ (`self.Health`) (`self.MaxHealth`)) 0.25)
    (`BlackboardComponent.SetValueAsBool` (`AIBlueprintHelperLibrary.GetBlackboard` null) "ActivateSpecial?" true)))

(fn `EvaluateScore`
  (bind _gm_cave_ref (`self.GM_Cave_Ref`))
  (for _array_element (`PrimitiveComponent.GetOverlappingActors` (`self.CapsuleComponent`) "/Script/Engine.TriggerVolume")
    (bind _tags (`Actor.Tags` _array_element))
    (if (and (`KismetArrayLibrary.Array_Contains` _tags "Red") (`self.IsRedSpider?`))
      _
      (elif (and (`KismetArrayLibrary.Array_Contains` _tags "Green") (not (`self.IsRedSpider?`)))
        _
        (else
          (`/Engine/EditorBlueprintResources/StandardMacros.IsValid` _gm_cave_ref
            (:`Is Valid`
              (`/Game/ClicheGame/Blueprints/GM_Cave.IncreaseScore` _gm_cave_ref 1))
            (:`Is Not Valid`
              _))
          (`self.K2_DestroyActor`)
          (return))))
    (`/Game/ClicheGame/Blueprints/GM_Cave.IncreaseScore` (`self.GM_Cave_Ref`) 3)
    (`self.K2_DestroyActor`)
    (return)))

(fn `UserConstructionScript`
  (`parent.UserConstructionScript`))