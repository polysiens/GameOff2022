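; BP_Wolf is the Forest Wolf NPC, a child Blueprint that adds wolf-specific setup and reactions to its parent.
; On BeginPlay it tints its NPC widget dark gray.
; Taking damage sets the "Interrupted?" blackboard key for its AI.
; DiesEffect plays a sped-up death animation in single-node mode, spawns a despawn particle slightly below the actor, then destroys it shortly after.
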(event `self.ReceiveBeginPlay`
  (`parent.ReceiveBeginPlay`)
  (bind _asw_npc_widget (cast `/Game/ClicheGame/Blueprints/UI/w_NPC_Widget` (`WidgetComponent.GetWidget` (`self.NPC_Widget`))))
  (`/Game/ClicheGame/Blueprints/UI/w_NPC_Widget.SetColor` _asw_npc_widget (struct :`R` 0.234551 :`G` 0.234551 :`B` 0.234551 :`A` 1.0)))

(event `self.ReceiveAnyDamage`
  (params (Damage :type "Float (single-precision)") (DamageType :type "DamageType Object Reference") (InstigatedBy :type "Controller Object Reference") (DamageCauser :type "Actor Object Reference"))
  (`parent.ReceiveAnyDamage` Damage DamageType InstigatedBy DamageCauser)
  (`BlackboardComponent.SetValueAsBool` (`AIBlueprintHelperLibrary.GetBlackboard` null) "Interrupted?" true))

(event `self.DiesEffect`
  (bind (_returnvalue_x _returnvalue_y _returnvalue_z) (`KismetMathLibrary.BreakVector` (`self.K2_GetActorLocation`)))
  (bind _mesh (`self.Mesh`))
  (`SkeletalMeshComponent.SetAnimationMode` _mesh "AnimationSingleNode")
  (`SkeletalMeshComponent.PlayAnimation` _mesh "/Game/ClicheGame/NPCs/Forest_Wolf/Wolf/Animations/ANIM_Wolf_Death.ANIM_Wolf_Death" false)
  (`SkeletalMeshComponent.SetPlayRate` _mesh 1.4)
  (`|ExecutionSequence`
    (:`then_0`
      (`KismetSystemLibrary.Delay` 1.0)
      (`self.K2_DestroyActor`))
    (:`then_1`
      (`KismetSystemLibrary.Delay` 0.7)
      (`GameplayStatics.SpawnEmitterAtLocation` "/Game/ClicheGame/Particles/Wukong/Particles/Wukong/Abilities/Ultimate/FX/p_CloneDespawn.p_CloneDespawn" (`KismetMathLibrary.MakeVector` _returnvalue_x _returnvalue_y (- _returnvalue_z 60.0))))))

(fn `UserConstructionScript`
  (`parent.UserConstructionScript`))