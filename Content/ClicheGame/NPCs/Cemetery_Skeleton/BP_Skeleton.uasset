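; BP_Skeleton is a skeleton NPC Blueprint for the cemetery level.
; On BeginPlay, if BasicSkeleton is set, it attaches a sword mesh to the hand-held SwordSocket, then tints its NPC widget white.
; DiesEffect plays a one-shot death animation, waits briefly, tells GM_Cemetery to update graves, and destroys the actor.
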(event `self.ReceiveBeginPlay`
  (`parent.ReceiveBeginPlay`)
  (`|ExecutionSequence`
    (:`then_0`
      (if (`self.BasicSkeleton?`)
        (bind _returnvalue (`AddComponent|NODE_AddSkeletalMeshComponent-0`))
        (`SceneComponent.K2_AttachToComponent` _returnvalue (`self.Mesh`) "SwordSocket" "SnapToTarget" "SnapToTarget" "KeepRelative" true)
        (`SkinnedMeshComponent.SetSkinnedAssetAndUpdate` _returnvalue "/Game/ClicheGame/NPCs/Cemetery_Skeleton/Corpse_Basic/enemy_Sword_Mesh.enemy_Sword_Mesh" false)))
    (:`then_1`
      (bind _asw_npc_widget (cast `/Game/ClicheGame/Blueprints/UI/w_NPC_Widget` (`WidgetComponent.GetWidget` (`self.NPC_Widget`))))
      (`/Game/ClicheGame/Blueprints/UI/w_NPC_Widget.SetColor` _asw_npc_widget (struct :`R` 1.0 :`G` 1.0 :`B` 1.0 :`A` 1.0)))))

(event `self.DiesEffect`
  (bind _mesh (`self.Mesh`))
  (`SkeletalMeshComponent.SetAnimationMode` _mesh "AnimationSingleNode")
  (`SkeletalMeshComponent.PlayAnimation` _mesh "/Game/ClicheGame/NPCs/Cemetery_Skeleton/Animation/Corpse_Alert_Death3.Corpse_Alert_Death3" false)
  (`KismetSystemLibrary.Delay` 0.7)
  (bind _asgm_cemetery (cast `/Game/ClicheGame/Blueprints/GM_Cemetery` (`GameplayStatics.GetGameMode`))
    (:`then`
      (`/Game/ClicheGame/Blueprints/GM_Cemetery.UpdateGraves` _asgm_cemetery))
    (:`CastFailed`
      _))
  (`self.K2_DestroyActor`))

(fn `UserConstructionScript`
  (`parent.UserConstructionScript`))