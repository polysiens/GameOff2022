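; BP_Grave is a destructible cemetery grave that can release a skeleton when broken.
; Damage plays a stone hit scaled in volume and lowers Health; at zero it destroys itself, first spawning an explosion and BP_Skeleton for three specific meshes.
; The construction script applies the chosen mesh and fits the Box to those three variants.
; BeginPlay starts audio if the priest beam is visible, and EndPlay tells GM_Cemetery to update graves.
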(event `self.ReceiveBeginPlay`
  (if (`SceneComponent.IsVisible` (`self.P_Priest_Beam`))
    (`AudioComponent.Play` (`self.Audio`) 0.0)))

(event `SpawnSkeleton`
  (bind _staticmesh (`StaticMeshComponent.StaticMesh` (`self.GraveMesh`)))
  (if (or (== _staticmesh "/Game/Cemetery_VOL1/Meshes/SM_Grave_Site_01a.SM_Grave_Site_01a") (== _staticmesh "/Game/Cemetery_VOL1/Meshes/SM_Grave_06a.SM_Grave_06a") (== _staticmesh "/Game/Cemetery_VOL1/Meshes/SM_Grave_05a.SM_Grave_05a"))
    (`GameplayStatics.SpawnEmitterAtLocation` "/Game/ClicheGame/Particles/Luos8Elements/Particles/Light/Par_4E_Light_Explosion_01.Par_4E_Light_Explosion_01" (`SceneComponent.K2_GetComponentLocation` (`self.Scene`)) (struct) (1.5 1.5 1.5))
    (`KismetSystemLibrary.Delay` 0.5)
    (`|SpawnActorFromClass` "/Game/ClicheGame/NPCs/Cemetery_Skeleton/BP_Skeleton.BP_Skeleton_C" (`self.GetTransform`) "AdjustIfPossibleButAlwaysSpawn" "OverrideRootScale" null true null))
  (`self.K2_DestroyActor`))

(event `self.ReceiveAnyDamage`
  (params (Damage :type "Float (single-precision)") (DamageType :type "DamageType Object Reference") (InstigatedBy :type "Controller Object Reference") (DamageCauser :type "Actor Object Reference"))
  (`GameplayStatics.PlaySoundAtLocation` "/Game/ClicheGame/Audio/SFX/Environment/Cue_StoneHit.Cue_StoneHit" (`self.K2_GetActorLocation`) (struct) (`KismetMathLibrary.MapRangeUnclamped` Damage 15.0 30.0 0.4 0.8) (`KismetMathLibrary.RandomFloatInRange` 0.9 1.1) 0.0 null null null null)
  (set `self.Health` (- (`self.Health`) (`KismetMathLibrary.FTrunc` Damage)))
  (if (<= (`self.Health`) 0)
    (`self.SpawnSkeleton`)))

(event `self.ReceiveEndPlay`
  (params (EndPlayReason :type "EEndPlayReason Enum" :default "Destroyed"))
  (bind _asgm_cemetery (cast `/Game/ClicheGame/Blueprints/GM_Cemetery` (`GameplayStatics.GetGameMode`)))
  (`/Game/ClicheGame/Blueprints/GM_Cemetery.UpdateGraves` _asgm_cemetery))

(fn `DoesHaveSkeleton`
  (returns (Bool :type Boolean))
  (bind _staticmesh (`StaticMeshComponent.StaticMesh` (`self.GraveMesh`)))
  (return (or (== _staticmesh "/Game/Cemetery_VOL1/Meshes/SM_Grave_Site_01a.SM_Grave_Site_01a") (== _staticmesh "/Game/Cemetery_VOL1/Meshes/SM_Grave_06a.SM_Grave_06a") (== _staticmesh "/Game/Cemetery_VOL1/Meshes/SM_Grave_05a.SM_Grave_05a"))))

(fn `UserConstructionScript`
  (bind _box (`self.Box`))
  (bind _staticmesh (`StaticMeshComponent.StaticMesh` (`self.GraveMesh`)))
  (`StaticMeshComponent.SetStaticMesh` (`self.GraveMesh`) (`self.StaticMesh`))
  (`|ExecutionSequence`
    (:`then_0`
      (if (== _staticmesh "/Game/Cemetery_VOL1/Meshes/SM_Grave_Site_01a.SM_Grave_Site_01a")
        (`SceneComponent.K2_SetRelativeLocation` _box (-91.131073 91.348534 118.475052) false false)
        (`SceneComponent.SetWorldScale3D` _box (2.573802 2.455103 3.494217))))
    (:`then_1`
      (if (== _staticmesh "/Game/Cemetery_VOL1/Meshes/SM_Grave_06a.SM_Grave_06a")
        (`SceneComponent.K2_SetRelativeLocation` _box (65.681969 119.795044 74.80986) false false)
        (`SceneComponent.SetWorldScale3D` _box (1.787258 3.274606 2.296131))))
    (:`then_2`
      (if (== _staticmesh "/Game/Cemetery_VOL1/Meshes/SM_Grave_05a.SM_Grave_05a")
        (`SceneComponent.K2_SetRelativeLocation` _box (0.0 0.0 91.698776) false false)
        (`SceneComponent.SetWorldScale3D` _box (2.053982 3.274606 2.80559))))))