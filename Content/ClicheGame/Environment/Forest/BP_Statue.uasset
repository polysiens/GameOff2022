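; Destructible forest statue that tracks health and reports its destruction to the forest game mode.
; Any damage plays a metal hit sound with volume scaled by damage and random pitch, then lowers Health.
; At zero or below it spawns a smoke burst, destroys itself a tick later and calls UpdateStatues on GM_Forest.
; Every hit, lethal or not, sends Health to all widgets implementing InteractionUI_Interface.
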(event `self.ReceiveAnyDamage`
  (params (Damage :type "Float (single-precision)") (DamageType :type "DamageType Object Reference") (InstigatedBy :type "Controller Object Reference") (DamageCauser :type "Actor Object Reference"))
  (bind _health (`self.Health`))
  (`GameplayStatics.PlaySoundAtLocation` "/Game/ClicheGame/Audio/SFX/Environment/MetalHit.MetalHit" (`self.K2_GetActorLocation`) (struct) (`KismetMathLibrary.MapRangeClamped` Damage 20.0 35.0 0.4 0.9) (`KismetMathLibrary.RandomFloatInRange` 1.1 1.4) 0.0 null null null null)
  (set `self.Health` (`KismetMathLibrary.FTrunc` (- (`self.Health`) Damage)))
  (if (<= _health 0)
    (`|ExecutionSequence`
      (:`then_0`
        (`GameplayStatics.SpawnEmitterAtLocation` "/Game/ClicheGame/Particles/P_FallenAngel_Ascend_HitSmoke.P_FallenAngel_Ascend_HitSmoke" (`self.K2_GetActorLocation`) (struct) (1.5 1.5 5.0))
        (`KismetSystemLibrary.DelayUntilNextTick`)
        (`self.K2_DestroyActor`)
        (bind _asgm_forest (cast `/Game/ClicheGame/Blueprints/GM_Forest` (`GameplayStatics.GetGameMode`)))
        (`/Game/ClicheGame/Blueprints/GM_Forest.UpdateStatues` _asgm_forest))
      (:`then_1`
        (bind _foundwidgets (`WidgetBlueprintLibrary.GetAllWidgetsWithInterface` "/Game/ClicheGame/Blueprints/Data/InteractionUI_Interface.InteractionUI_Interface_C" :!label _label))
        (for _array_element _foundwidgets
          (message `/Game/ClicheGame/Blueprints/Data/InteractionUI_Interface.StructureDamage` _array_element _health))))
    (else
      (goto _label))))

(fn `UserConstructionScript`)